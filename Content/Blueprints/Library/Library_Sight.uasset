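; Blueprint function library for sight checks, with one function that tests whether a target actor is on the first player's screen.
; IsActorOnScreen projects the target's location to screen space and compares it with the viewport bounds, also returning its 2D pixel distance from screen center.
; The upper width check compares screen Y instead of X, so the right edge goes untested.
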(fn `IsActorOnScreen`
  (params (Instigator :type "Character Object Reference") (Target :type "Actor Object Reference"))
  (returns (OnScreen :type Boolean) (Offset :type "Float (double-precision)"))
  (bind _returnvalue (`WidgetLayoutLibrary.GetViewportSize` Instigator))
  (bind _screenlocation (`PlayerController.ProjectWorldLocationToScreen` (`GameplayStatics.GetPlayerController` Instigator) (`Actor.K2_GetActorLocation` Target) false))
  (bind (_x _y) (`KismetMathLibrary.BreakVector2D` _returnvalue))
  (bind (_x_2 _y_2) (`KismetMathLibrary.BreakVector2D` _screenlocation))
  (return (and (> _x_2 0.0) (> _y_2 0.0) (< _y_2 _x) (< _y_2 _y)) (`KismetMathLibrary.Distance2D` _screenlocation (* _returnvalue 0.5))))
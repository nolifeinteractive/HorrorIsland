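; Base ability Blueprint that provides a timer-based cooldown.
; Fire starts a timer by function name for the Cooldown duration, which calls AbilityAvailable to print a reset message.
; GetCooldownTimeRemaining queries that timer for remaining seconds and a fraction of Cooldown, selecting zero when inactive.
; Update calls this query without using the result, Fire has no cooldown check, and both debug events are empty stubs.
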(event `Update`
  (params (Instigator :type "Character Object Reference"))
  (`self.GetCooldownTimeRemaining`))

(event `Fire`
  (`KismetSystemLibrary.K2_SetTimer` self "AbilityAvailable" (`self.Cooldown`)))

(event `AbilityAvailable`
  (`KismetSystemLibrary.PrintString` null "ABILITY RESET"))

(event `DebugUpdate`)

(event `DebugLog`)

(fn `GetCooldownTimeRemaining`
  (returns (Remaining :type "Float (double-precision)") (Factor :type "Float (double-precision)"))
  (bind _returnvalue (`KismetSystemLibrary.K2_GetTimerRemainingTime` self "AbilityAvailable"))
  (bind _returnvalue_2 (`KismetSystemLibrary.K2_IsTimerActive` self "AbilityAvailable"))
  (return (`KismetMathLibrary.SelectFloat` _returnvalue 0.0 _returnvalue_2) (`KismetMathLibrary.SelectFloat` (/ _returnvalue (`self.Cooldown`)) 0.0 _returnvalue_2)))
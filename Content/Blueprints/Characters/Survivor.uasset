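; Survivor character Blueprint that detects when the monster is on screen and tracks a Sanity value.
; Each tick it gets the Monster from LobbyGM, runs an on-screen check against it and, when visible, calls the monster's Seen with itself and the screen offset.
; ModifySanity adds to Sanity and refreshes the sanity debug display through player 0's LobbyPC.
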(event `self.ReceiveTick`
  (params (DeltaSeconds :type "Float (single-precision)"))
  (bind _aslobby_gm (cast `/Game/Blueprints/Lobby/LobbyGM` (`GameplayStatics.GetGameMode`)))
  (bind _monster (`/Game/Blueprints/Lobby/LobbyGM.Monster` _aslobby_gm))
  (`/Engine/EditorBlueprintResources/StandardMacros.IsValid` _monster
    (:`Is Valid`
      (bind (_onscreen _offset) (`/Game/Blueprints/Library/Library_Sight.IsActorOnScreen` self _monster))
      (if _onscreen
        (`self.Seen` _monster self _offset)))))

(event `self.ModifySanity`
  (params (Value :type "Float (single-precision)"))
  (set `self.Sanity` (+ (`self.Sanity`) Value))
  (bind _aslobby_pc (cast `/Game/Blueprints/Lobby/LobbyPC` (`GameplayStatics.GetPlayerController` 0)))
  (`/Game/Blueprints/Lobby/LobbyPC.UpdateSanityDebug` _aslobby_pc self))

(fn `UserConstructionScript`
  (`parent.UserConstructionScript`))